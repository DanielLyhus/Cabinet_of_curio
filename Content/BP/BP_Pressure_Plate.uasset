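; BP_Pressure_Plate is a pressure plate that completes when a rock is placed on it.
; When an actor whose root component carries the Rock tag overlaps the Box, a DoOnce lets the response fire a single time.
; The plate mesh drops, turns green and plays a sound, then the Complete flag is set and the PressurePlateComplete dispatcher is called to notify listeners.
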(event OnComponentBeginOverlap(Box)
  (params (OverlappedComponent :type Primitive%20Component%20Object%20Reference) (OtherActor :type Actor%20Object%20Reference) (OtherComp :type Primitive%20Component%20Object%20Reference) (OtherBodyIndex :type Integer) (bFromSweep :type Boolean) (SweepResult :type Hit%20Result%20Structure%20%28by%20ref%29))
  (if (Components|ComponentHasTag (Variables|/Script/Engine.Actor|GetRootComponent OtherActor) "Rock")
    (Utilities|FlowControl|DoOnce false
      (:Completed
        (Transformation|AddLocalOffset (Variables|Default|GetCube1) "0.000000,0.000000,-50.000000" false false)
        (Audio|PlaySound2D "/Game/BP/chrisiex1-correct-156911__1_.chrisiex1-correct-156911__1_" 1.0 1.0 0.0 0 0)
        (Rendering|Material|SetMaterial (Variables|Default|GetCube1) 0 "/Game/BP/M_Green.M_Green")
        (Variables|Default|SetComplete true)
        (Default|CallPressurePlateComplete)))))

(event EventBeginPlay)

(event Collision|EventActorBeginOverlap
  (params (OtherActor :type Actor%20Object%20Reference)))

(event EventTick
  (params (DeltaSeconds :type Float%20%28single-precision%29)))

(fn ConstructionScript)