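; Rock dropper station that lets the first-person player position a rock and release it, with input enabled while overlapping it.
; E alternates between spawning a gravity-less BP_Rock while freezing player movement, and dropping it, then restoring movement, the display rock and later destroying the spawn.
; A and D shift the target along clamped world X, swappable via ReverseDirection, and a Tick-fed Gate pins the rock there until release.
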(event EventBeginPlay)

(event EventTick
  (params (DeltaSeconds :type Float%20%28single-precision%29))
  (Utilities|FlowControl|Gate true
    (:Exit
      (Transformation|SetWorldLocation (Variables|/Game/BP/BP_Rock.BP_Rock_C|GetSphere (stale Input|KeyboardEvents|E _returnvalue_2)) (stale Input|KeyboardEvents|E _output_get) false false))))

(event Collision|EventActorBeginOverlap
  (params (OtherActor :type Actor%20Object%20Reference))
  (Utilities|Casting|CastToBP_FirstPersonCharacter OtherActor)
  (Input|EnableInput (Game|GetPlayerController 0)))

(event Collision|EventActorEndOverlap
  (params (OtherActor :type Actor%20Object%20Reference))
  (Utilities|Casting|CastToBP_FirstPersonCharacter OtherActor)
  (Input|DisableInput (Game|GetPlayerController 0)))

(event Input|MouseEvents|LeftMouseButton
  (params (Key :type Key%20Structure :default "None")))

(event Input|KeyboardEvents|E
  (params (Key :type Key%20Structure :default "None"))
  (bind _returnvalue (Game|GetPlayerCharacter 0))
  (bind _rock (Variables|Default|GetRock))
  (bind _charactermovement (Variables|/Script/Engine.Character|GetCharacterMovement _returnvalue))
  (:Pressed
    (Development|SetHiddeninGame _rock true false)
    (Utilities|FlowControl|FlipFlop
      (:A
        (Utilities|FlowControl|DoOnce false :!label _label
          (:Completed
            (Input|EnableInput (Game|GetPlayerController 0))
            (bind _returnvalue_2 (Game|SpawnActorfromClass "/Game/BP/BP_Rock.BP_Rock_C" (Transformation|GetWorldTransform (Variables|Default|GetRock%20place)) "Undefined" "MultiplyWithRoot" 0 0))
            (Physics|SetEnableGravity (Variables|/Game/BP/BP_Rock.BP_Rock_C|GetSphere _returnvalue_2) false)
            (Pawn|Components|CharacterMovement|DisableMovement _charactermovement)
            (bind _output_get (Variables|Default|SetStart%20Location_Ball (Transformation|GetWorldLocation (Variables|/Game/BP/BP_Rock.BP_Rock_C|GetSphere _returnvalue_2))))
            (Utilities|FlowControl|Gate true) ; enters at Open
          )))
      (:B
        (Physics|SetEnableGravity (Variables|/Game/BP/BP_Rock.BP_Rock_C|GetSphere _returnvalue_2) true)
        (Utilities|FlowControl|Sequence
          (:then_0
            (Utilities|FlowControl|Gate true) ; enters at Close
          )
          (:then_1
            (Utilities|FlowControl|Delay 0.25)
            (Pawn|Components|CharacterMovement|SetMovementMode _charactermovement "MOVE_Walking" 0)
            (Utilities|FlowControl|Delay 1.0)
            (Development|SetHiddeninGame _rock false false)
            (goto _label Reset))
          (:then_2
            (Utilities|FlowControl|Delay 6e+01)
            (Actor|DestroyActor _returnvalue_2)))))))

(event Input|KeyboardEvents|A
  (params (Key :type Key%20Structure :default "None"))
  (bind _rock_place (Variables|Default|GetRock%20place))
  (bind _returnvalue (Transformation|GetWorldLocation _rock_place))
  (bind _returnvalue_2 (+ (.x _returnvalue) -3e+02))
  (bind _returnvalue_3 (+ (.x _returnvalue) 3e+02))
  (:Pressed
    (if (Variables|Default|GetReverse_Direction)
      (Variables|Default|SetStart%20Location_Ball (Math|Vector|MakeVector (Math|Float|Clamp(Float) (+ (.x (Variables|Default|GetStart%20Location_Ball)) 5e+01) _returnvalue_2 _returnvalue_3) (.y (Variables|Default|GetStart%20Location_Ball)) (.z (Variables|Default|GetStart%20Location_Ball))))
      (else
        (Variables|Default|SetStart%20Location_Ball (Math|Vector|MakeVector (Math|Float|Clamp(Float) (+ (.x (Variables|Default|GetStart%20Location_Ball)) -5e+01) _returnvalue_2 _returnvalue_3) (.y (Variables|Default|GetStart%20Location_Ball)) (.z (Variables|Default|GetStart%20Location_Ball))))))))

(event Input|KeyboardEvents|D
  (params (Key :type Key%20Structure :default "None"))
  (bind _rock_place (Variables|Default|GetRock%20place))
  (bind _returnvalue (Transformation|GetWorldLocation _rock_place))
  (bind _returnvalue_2 (+ (.x _returnvalue) -3e+02))
  (bind _returnvalue_3 (+ (.x _returnvalue) 3e+02))
  (:Pressed
    (if (Variables|Default|GetReverse_Direction)
      (Variables|Default|SetStart%20Location_Ball (Math|Vector|MakeVector (Math|Float|Clamp(Float) (+ (.x (Variables|Default|GetStart%20Location_Ball)) -5e+01) _returnvalue_2 _returnvalue_3) (.y (Variables|Default|GetStart%20Location_Ball)) (.z (Variables|Default|GetStart%20Location_Ball))))
      (else
        (Variables|Default|SetStart%20Location_Ball (Math|Vector|MakeVector (Math|Float|Clamp(Float) (+ (.x (Variables|Default|GetStart%20Location_Ball)) 5e+01) _returnvalue_2 _returnvalue_3) (.y (Variables|Default|GetStart%20Location_Ball)) (.z (Variables|Default|GetStart%20Location_Ball))))))))

(fn ConstructionScript)