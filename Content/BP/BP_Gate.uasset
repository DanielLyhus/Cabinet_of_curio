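; Gate actor whose mesh rises while its GateController reports IsOpening and otherwise drops faster.
; Tick steps the height between hard-coded world Z limits, setting GateMaxHeight and GateClosed flags.
; HasOpened arms a one-shot slam sound for when the falling gate nears the bottom.
; Near the top, the closing branch joins the opening path, so the gate keeps rising instead of dropping.
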(event EventBeginPlay
  (bind _sm_gate (Variables|Default|GetSM_Gate))
  (bind _returnvalue (Transformation|GetWorldLocation _sm_gate))
  (bind (_x _y _z) (Math|Vector|BreakVector _returnvalue))
  (Variables|Default|SetStart%20Location _returnvalue)
  (Variables|Default|SetEnd%20Location (Math|Vector|MakeVector _x _y (+ _z 5e+02))))

(event EventTick
  (params (DeltaSeconds :type Float%20%28single-precision%29))
  (bind _sm_gate (Variables|Default|GetSM_Gate))
  (bind _sm_gate_2 (Variables|Default|GetSM_Gate))
  (bind _sm_gate_3 (Variables|Default|GetSM_Gate))
  (bind _returnvalue (Transformation|GetWorldLocation _sm_gate))
  (bind _returnvalue_2 (Transformation|GetWorldLocation _sm_gate_2))
  (bind _returnvalue_3 (+ (.z _returnvalue_2) -5.0))
  (bind _returnvalue_4 (+ (.z _returnvalue_2) 1.0))
  (bind _returnvalue_5 (Math|Float|Clamp(Float) _returnvalue_3 4e+02 1e+03))
  (bind _returnvalue_6 (Math|Float|Clamp(Float) _returnvalue_4 0.0 1e+03))
  (bind _returnvalue_7 (Math|Vector|MakeVector (.x _returnvalue_2) (.y _returnvalue_2) _returnvalue_5))
  (if (Variables|/Game/BP/BP_Gate_Controller.BP_Gate_Controller_C|GetIs%20Opening (Variables|Default|GetGate%20Controller))
    (if (>= (.z _returnvalue) 6e+02)
      (bind _output_get (Variables|Default|SetHas_Opened true)))
    (if (>= _returnvalue_6 9.5e+02)
      (Variables|Default|SetGate_max_height true :!label _label)
      (else
        (Variables|Default|SetGate_max_height false)))
    (Variables|Default|SetGate_Closed false)
    (Transformation|SetWorldLocation _sm_gate_3 (Math|Vector|MakeVector (.x _returnvalue_2) (.y _returnvalue_2) _returnvalue_6) false false)
    (else
      (if (< (.z _returnvalue) 425.0)
        (if _output_get
          (Audio|PlaySound2D "/Game/soundreality-metal-door-slam-172172.soundreality-metal-door-slam-172172" 1.0 1.0 0.0 0 0)
          (Variables|Default|SetHas_Opened false)))
      (if (>= _returnvalue_5 9.5e+02)
        (goto _label)
        (else
          (Variables|Default|SetGate_max_height false)
          (if (Utilities|Operators|EqualEqual _returnvalue_7 (Variables|Default|GetStart%20Location) 5.0)
            (Variables|Default|SetGate_Closed true))
          (Transformation|SetWorldLocation _sm_gate_3 _returnvalue_7 false false))))))

(fn ConstructionScript)