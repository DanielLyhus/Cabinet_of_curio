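; Three-stage code lock puzzle that opens a stone door, operated by the player while inside its trigger box.
; E toggles between the puzzle camera and walking, handing input to the active BP_Code_Wheel child actor.
; Left click checks its number against Solution (currently always 0); success carries the number to the next wheel while a timeline slides the track.
; The final solve returns control and swings the door with sound, dust and camera shake.
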(event OnComponentBeginOverlap(Box)
  (params (OverlappedComponent :type Primitive%20Component%20Object%20Reference) (OtherActor :type Actor%20Object%20Reference) (OtherComp :type Primitive%20Component%20Object%20Reference) (OtherBodyIndex :type Integer) (bFromSweep :type Boolean) (SweepResult :type Hit%20Result%20Structure%20%28by%20ref%29))
  ;[1 1 1] Box Overlap enable input
  (Utilities|Casting|CastToBP_FirstPersonCharacter OtherActor)
  (Input|EnableInput (Game|GetPlayerController 0)))

(event OnComponentEndOverlap(Box)
  (params (OverlappedComponent :type Primitive%20Component%20Object%20Reference) (OtherActor :type Actor%20Object%20Reference) (OtherComp :type Primitive%20Component%20Object%20Reference) (OtherBodyIndex :type Integer))
  ;[1 1 1] Box Overlap enable input
  (Utilities|Casting|CastToBP_FirstPersonCharacter OtherActor)
  (Input|DisableInput (Game|GetPlayerController 0)))

(event EventBeginPlay
  ;[1 1 1] Initialize Stuff
  (Input|DisableInput (Game|GetPlayerController 0))
  (CallFunction|SetTrackLocation)
  (Variables|Default|SetCurrentCodeWheelActor (Variables|Default|GetBP_Code_Wheel_1))
  (Variables|Default|SetSolution 0)
  (Variables|Default|SetDoor%20Rotation (Variables|/Script/Engine.SceneComponent|GetRelativeRotation (Variables|Default|GetBP_Code_Door))))

(event EventTick
  (params (DeltaSeconds :type Float%20%28single-precision%29))
  ;[1 1 1] Debug solution
  (Development|PrintString (Utilities|String|ToString(Integer) (Variables|Default|GetSolution)) true true "(R=0.000000,G=0.660000,B=1.000000,A=1.000000)" 2.0 "wadadawda"))

(event Input|MouseEvents|LeftMouseButton
  (params (Key :type Key%20Structure :default "None"))
  (bind _returnvalue (Transformation|GetActorLocation))
  (bind _door_rotation (Variables|Default|GetDoor%20Rotation))
  (bind _active (Variables|Default|GetActive))
  (bind _active_2 (Variables|Default|GetActive))
  (bind _active_3 (Variables|Default|GetActive))
  ;[1 1 1] Checks against solution
  (:Pressed
    (Development|PrintString (Utilities|String|ToString(Integer) (Variables|/Game/BP/Code_V2/BP_Code_Wheel.BP_Code_Wheel_C|GetCurrent_Number (Variables|Default|GetActive))))
    (if (== (Variables|/Game/BP/Code_V2/BP_Code_Wheel.BP_Code_Wheel_C|GetCurrent_Number (Variables|Default|GetActive)) (Variables|Default|GetSolution))
      ;[1 1 1] Moves to next number when solved
      (Utilities|FlowControl|DoOnce false :!label _label
        (:Completed
          (if (Variables|Default|Get1Solved?)
            (if (Variables|Default|Get2Solved?)
              (if (Variables|Default|Get2Solved?)
                (CallFunction|SetDisabled (Variables|Default|GetCurrentCodeWheelActor))
                (Default|Solved (Variables|Default|GetActive))
                (Game|Player|SetViewTargetwithBlend (Game|GetPlayerController 0) (Game|GetPlayerCharacter 0) (Variables|Default|GetBlend%20Time%20Camera) "VTBlend_Linear" 0.0 false)
                (CallFunction|SetDisabled (Variables|Default|GetCurrentCodeWheelActor))
                (Utilities|FlowControl|Delay 0.25)
                (Pawn|Components|CharacterMovement|SetMovementMode (Variables|/Script/Engine.Character|GetCharacterMovement (Game|GetPlayerCharacter 0)) "MOVE_Walking" 0)
                ;[1 1 1] Door opening animation
                (Audio|PlaySoundatLocation "/Game/BP/Code_V2/Misc/krnbeatz-tectonic-passage-418836.krnbeatz-tectonic-passage-418836" _returnvalue "0, 0, 0" 0.4 1.0 0.0 0 0 0 0)
                (Audio|PlaySoundatLocation "/Game/BP/Code_V2/Misc/freesound_community-stoneblockdragwoodgrind-82327.freesound_community-stoneblockdragwoodgrind-82327" "0, 0, 0" "0, 0, 0" 0.4 0.5 -1.0 0 0 0 0)
                (Camera|PlayWorldCameraShake "/Game/BP/Code_V2/Misc/CS_Door.CS_Door_C" _returnvalue 0.0 1e+03)
                (Components|Activation|SetActive (Variables|Default|GetNS_Dust2) true false)
                (bind (_direction _newtrack_0 _newtrack_1) (Timeline|Timeline_1 PlayFromStart)
                  (:Update
                    (Transformation|SetRelativeRotation (Variables|Default|GetBP_Code_Door) (Math|Rotator|MakeRotator (.roll _door_rotation) (.pitch _door_rotation) (+ (* _newtrack_0 -9e+01) (.yaw _door_rotation))) false false)
                    (Transformation|AddLocalOffset (Variables|Default|GetBP_Code_Wheel_3) (Math|Vector|MakeVector 0.0 (* _newtrack_1 -0.7) 0.0) false false))
                  (:Finished
                    (Components|Activation|SetActive (Variables|Default|GetNS_Dust) false false))))
              (else
                (Variables|Default|SetConsistentNumber (Variables|/Game/BP/Code_V2/BP_Code_Wheel.BP_Code_Wheel_C|GetCurrent_Number (Variables|Default|GetActive)))
                (CallFunction|SetDisabled (Variables|Default|GetCurrentCodeWheelActor))
                (Default|Solved (Variables|Default|GetActive))
                (bind _output_get (Variables|Default|SetCurrentCodeWheelActor (Variables|Default|GetBP_Code_Wheel_3)))
                (CallFunction|SetActive _output_get)
                (Variables|/Game/BP/Code_V2/BP_Code_Wheel.BP_Code_Wheel_C|SetCurrent_Number _active (Variables|Default|GetConsistentNumber))
                (Default|UpdateDials _active)
                (bind _wheel_change (Timeline|Timeline_0 PlayFromStart)
                  (:Update
                    (CallFunction|MoveTrack _wheel_change))
                  (:Finished
                    (Variables|Default|Set2Solved? true)
                    (Variables|Default|SetSolution 0)
                    (CallFunction|SetTrackLocation)
                    (Utilities|FlowControl|Delay 1.5)
                    (goto _label Reset)))))
            (else
              (Variables|Default|SetConsistentNumber (Variables|/Game/BP/Code_V2/BP_Code_Wheel.BP_Code_Wheel_C|GetCurrent_Number _active_3))
              (CallFunction|SetDisabled (Variables|Default|GetCurrentCodeWheelActor))
              (Default|Solved _active_3)
              (bind _output_get_2 (Variables|Default|SetCurrentCodeWheelActor (Variables|Default|GetBP_Code_Wheel_2)))
              (CallFunction|SetActive _output_get_2)
              (Variables|/Game/BP/Code_V2/BP_Code_Wheel.BP_Code_Wheel_C|SetCurrent_Number _active_2 (Variables|Default|GetConsistentNumber))
              (Default|UpdateDials _active_2)
              (bind _wheel_change_2 (Timeline|Timeline PlayFromStart)
                (:Update
                  (CallFunction|MoveTrack _wheel_change_2))
                (:Finished
                  (Variables|Default|Set1Solved? true)
                  (Variables|Default|SetSolution 0)
                  (CallFunction|SetTrackLocation)
                  (Utilities|FlowControl|Delay 1.5)
                  (goto _label Reset)))))))
      (else
        ;[1 1 1] Wrong
        (Default|Wrong (Variables|Default|GetActive))))))

(event Input|KeyboardEvents|E
  (params (Key :type Key%20Structure :default "None"))
  (bind _returnvalue (Game|GetPlayerController 0))
  (bind _returnvalue_2 (Game|GetPlayerCharacter 0))
  (bind _currentcodewheelactor (Variables|Default|GetCurrentCodeWheelActor))
  ;[1 1 1] Use Code and update Camera With E
  (:Pressed
    (Utilities|FlowControl|FlipFlop
      (:A
        (Pawn|Components|CharacterMovement|DisableMovement (Variables|/Script/Engine.Character|GetCharacterMovement _returnvalue_2))
        (Game|Player|SetViewTargetwithBlend _returnvalue self (Variables|Default|GetBlend%20Time%20Camera) "VTBlend_Linear" 0.0 false)
        (CallFunction|SetActive _currentcodewheelactor))
      (:B
        (Game|Player|SetViewTargetwithBlend _returnvalue _returnvalue_2 (Variables|Default|GetBlend%20Time%20Camera) "VTBlend_Linear" 0.0 false)
        (CallFunction|SetDisabled _currentcodewheelactor)
        (Utilities|FlowControl|Delay 0.25)
        (Pawn|Components|CharacterMovement|SetMovementMode (Variables|/Script/Engine.Character|GetCharacterMovement (Game|GetPlayerCharacter 0)) "MOVE_Walking" 0)))))

(fn ConstructionScript)

(fn SetActive
  (params (Code_Wheel_Actor :type Child%20Actor%20Component%20Object%20Reference))
  (Variables|Default|SetCurrent_Wheel (+ 1 (Variables|Default|GetCurrent_Wheel)))
  (bind _asbp_code_wheel (Utilities|Casting|CastToBP_Code_Wheel (Variables|/Script/Engine.ChildActorComponent|GetChildActor Code_Wheel_Actor)))
  (bind _output_get (Variables|Default|SetActive _asbp_code_wheel))
  (Input|EnableInput _output_get (Game|GetPlayerController 0)))

(fn SetDisabled
  (params (Code_Wheel_Actor :type Child%20Actor%20Component%20Object%20Reference))
  (bind _asbp_code_wheel (Utilities|Casting|CastToBP_Code_Wheel (Variables|/Script/Engine.ChildActorComponent|GetChildActor Code_Wheel_Actor)))
  (Input|DisableInput _asbp_code_wheel (Game|GetPlayerController 0)))

(fn MoveTrack
  (params (Wheel_Movement :type Float%20%28double-precision%29))
  (bind _track_location (Variables|Default|GetTrack_Location))
  (Transformation|SetRelativeLocation (Variables|Default|GetTrack) (Math|Vector|MakeVector (+ (.x _track_location) (* Wheel_Movement 8e+01)) (.y _track_location) (.z _track_location)) false false))

(fn SetTrackLocation
  (Variables|Default|SetTrack_Location (Variables|/Script/Engine.SceneComponent|GetRelativeLocation (Variables|Default|GetTrack))))