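; Two-ring combination code wheel that dials a number from 0 to 99, with tens and ones on separate rings.
; Move input or mouse wheel steps the number through DoOnce gates, which reset after a delay to throttle input.
; Update_Dials converts each digit to a target rotation that Tick eases toward with RInterpTo.
; Solved and Wrong events give scale, sound and camera shake feedback; Wrong restores scale afterwards.
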(event Custom|Update_Dials
  (Utilities|FlowControl|Sequence
    (:then_0
      (Variables|Default|SetInterp%20Speed 4.0))
    (:then_1
      ;[1 1 1] Sets 01s
      (Variables|Default|SetTargetRotation2 (Math|Rotator|MakeRotator (* (- (Variables|Default|GetCurrent_Number) (* (Math|Float|Floor (* (Math|Conversions|ToFloat(Integer) (Variables|Default|GetCurrent_Number)) 0.1)) 10)) -36.0) 0.0 0.0))
      ;[1 1 1] Sets Roatation Based on 10s
      (bind _output_get (Variables|Default|SetTargetRotation1 (Math|Rotator|MakeRotator (* (Math|Float|Floor (* (Math|Conversions|ToFloat(Integer) (Variables|Default|GetCurrent_Number)) 0.1)) -36.0) 0.0 0.0)))
      ;[1 1 1] Delays next input
      (Utilities|FlowControl|Delay (Variables|Default|GetTime%20Between%20Inputs))
      (Utilities|FlowControl|Sequence
        (:then_0
          (Utilities|FlowControl|DoOnce false) ; enters at Reset
        )
        (:then_1
          (Utilities|FlowControl|DoOnce false) ; enters at Reset
        )))
    (:then_2
      (Utilities|FlowControl|Delay 2.0)
      (Variables|Default|SetInterp%20Speed 6.0))))

(event Custom|Solved
  ;[1 1 1] Solved Scale Change
  (Transformation|SetRelativeScale3D (Variables|Default|GetBP_Code_Ring_2) "0.800000,0.800000,0.800000")
  (Audio|PlaySound2D "/Game/BP/Code_V2/Misc/daviddumaisaudio-steampunk-gadget-lock-and-unlock-188053.daviddumaisaudio-steampunk-gadget-lock-and-unlock-188053" 1.0 1.0 0.0 0 0)
  (Camera|PlayWorldCameraShake "/Game/BP/Code_V2/Misc/CS_Correct.CS_Correct_C" (Transformation|GetActorLocation) 0.0 5e+02))

(event Custom|Wrong
  ;[1 1 1] Wrong changes
  (Transformation|SetRelativeScale3D (Variables|Default|GetBP_Code_Ring_2) "0.900000,0.900000,0.900000")
  (Audio|PlaySound2D "/Game/BP/Code_V2/Misc/soundreality-button-3-214381.soundreality-button-3-214381" 1.0 1.0 0.0 0 0)
  (Camera|PlayWorldCameraShake "/Game/BP/Code_V2/Misc/CS_Wrong.CS_Wrong_C" (Transformation|GetActorLocation) 0.0 5e+02)
  (Utilities|FlowControl|Delay 1.0)
  (Transformation|SetRelativeScale3D (Variables|Default|GetBP_Code_Ring_2) "1.000000,1.000000,1.000000"))

(event Input|EnhancedActionEvents|EnhancedInputActionIA_Move
  (params (ActionValue :type Vector%202D%20Structure) (ElapsedSeconds :type Float%20%28double-precision%29) (TriggeredSeconds :type Float%20%28double-precision%29) (InputAction :type Input%20Action%20Object%20Reference :default "/Game/FirstPerson/Input/Actions/IA_Move.IA_Move"))
  (if (== (.y ActionValue) 1.0)
    (Utilities|FlowControl|DoOnce false :!label _label
      (:Completed
        (Audio|PlaySound2D "/Game/BP/justsomesounds-click-sound-432501.justsomesounds-click-sound-432501" 0.5 (Math|Random|RandomFloatinRange 0.95 1.05) 0.2 0 0)
        ;[1 1 1] Sets Current Number
        (Variables|Default|SetCurrent_Number (Math|Integer|Clamp(Integer) (+ (Variables|Default|GetCurrent_Number) 1) 0 99))))
    (else
      (Utilities|FlowControl|DoOnce false :!label _label_2
        (:Completed
          (Audio|PlaySound2D "/Game/BP/justsomesounds-click-sound-432501.justsomesounds-click-sound-432501" 0.5 (Math|Random|RandomFloatinRange 0.9 0.8) 0.2 0 0)
          (Variables|Default|SetCurrent_Number (Math|Integer|Clamp(Integer) (+ (Variables|Default|GetCurrent_Number) -1) 0 99))))))
  ;[1 1 1] Sets 01s
  (Variables|Default|SetTargetRotation2 (Math|Rotator|MakeRotator (* (- (Variables|Default|GetCurrent_Number) (* (Math|Float|Floor (* (Math|Conversions|ToFloat(Integer) (Variables|Default|GetCurrent_Number)) 0.1)) 10)) -36.0) 0.0 0.0))
  ;[1 1 1] Sets Roatation Based on 10s
  (bind _output_get (Variables|Default|SetTargetRotation1 (Math|Rotator|MakeRotator (* (Math|Float|Floor (* (Math|Conversions|ToFloat(Integer) (Variables|Default|GetCurrent_Number)) 0.1)) -36.0) 0.0 0.0)))
  ;[1 1 1] Delays next input
  (Utilities|FlowControl|Delay (Variables|Default|GetTime%20Between%20Inputs))
  (Utilities|FlowControl|Sequence
    (:then_0
      (goto _label_2 Reset))
    (:then_1
      (goto _label Reset))))

(event Collision|EventActorBeginOverlap
  (params (OtherActor :type Actor%20Object%20Reference)))

(event EventTick
  (params (DeltaSeconds :type Float%20%28single-precision%29))
  (bind _interp_speed (Variables|Default|GetInterp%20Speed))
  ;[1 1 1] Rotates Dials
  (Transformation|SetRelativeRotation (Variables|Default|GetBP_Code_Ring_1) (Math|Interpolation|RInterpTo (Variables|/Script/Engine.SceneComponent|GetRelativeRotation (Variables|Default|GetBP_Code_Ring_1)) (stale Custom|Update_Dials _output_get) DeltaSeconds _interp_speed) false false)
  (Transformation|SetRelativeRotation (Variables|Default|GetBP_Code_Ring_2) (Math|Interpolation|RInterpTo (Variables|/Script/Engine.SceneComponent|GetRelativeRotation (Variables|Default|GetBP_Code_Ring_2)) (Variables|Default|GetTargetRotation2) DeltaSeconds _interp_speed) false false))

(event Input|MouseEvents|MouseWheelDown
  (params (Key :type Key%20Structure :default "None"))
  (:Pressed
    (Utilities|FlowControl|DoOnce false :!label _label
      (:Completed
        (Audio|PlaySound2D "/Game/BP/justsomesounds-click-sound-432501.justsomesounds-click-sound-432501" 0.5 (Math|Random|RandomFloatinRange 0.9 0.8) 0.2 0 0)
        ;[1 1 1] Sets Current Number
        (Variables|Default|SetCurrent_Number (Math|Integer|Clamp(Integer) (+ (Variables|Default|GetCurrent_Number) -1) 0 99))
        ;[1 1 1] Sets 01s
        (Variables|Default|SetTargetRotation2 (Math|Rotator|MakeRotator (* (- (Variables|Default|GetCurrent_Number) (* (Math|Float|Floor (* (Math|Conversions|ToFloat(Integer) (Variables|Default|GetCurrent_Number)) 0.1)) 10)) -36.0) 0.0 0.0))
        ;[1 1 1] Sets Roatation Based on 10s
        (bind _output_get (Variables|Default|SetTargetRotation1 (Math|Rotator|MakeRotator (* (Math|Float|Floor (* (Math|Conversions|ToFloat(Integer) (Variables|Default|GetCurrent_Number)) 0.1)) -36.0) 0.0 0.0)))
        ;[1 1 1] Delays next input
        (Utilities|FlowControl|Delay (Variables|Default|GetTime%20Between%20Inputs))
        (Utilities|FlowControl|Sequence
          (:then_0
            (goto _label Reset))
          (:then_1
            (Utilities|FlowControl|DoOnce false) ; enters at Reset
          ))))))

(event Input|MouseEvents|MouseWheelUp
  (params (Key :type Key%20Structure :default "None"))
  (:Pressed
    (Utilities|FlowControl|DoOnce false :!label _label
      (:Completed
        (Audio|PlaySound2D "/Game/BP/justsomesounds-click-sound-432501.justsomesounds-click-sound-432501" 0.5 (Math|Random|RandomFloatinRange 0.95 1.05) 0.2 0 0)
        ;[1 1 1] Sets Current Number
        (Variables|Default|SetCurrent_Number (Math|Integer|Clamp(Integer) (+ (Variables|Default|GetCurrent_Number) 1) 0 99))
        ;[1 1 1] Sets 01s
        (Variables|Default|SetTargetRotation2 (Math|Rotator|MakeRotator (* (- (Variables|Default|GetCurrent_Number) (* (Math|Float|Floor (* (Math|Conversions|ToFloat(Integer) (Variables|Default|GetCurrent_Number)) 0.1)) 10)) -36.0) 0.0 0.0))
        ;[1 1 1] Sets Roatation Based on 10s
        (bind _output_get (Variables|Default|SetTargetRotation1 (Math|Rotator|MakeRotator (* (Math|Float|Floor (* (Math|Conversions|ToFloat(Integer) (Variables|Default|GetCurrent_Number)) 0.1)) -36.0) 0.0 0.0)))
        ;[1 1 1] Delays next input
        (Utilities|FlowControl|Delay (Variables|Default|GetTime%20Between%20Inputs))
        (Utilities|FlowControl|Sequence
          (:then_0
            (Utilities|FlowControl|DoOnce false) ; enters at Reset
          )
          (:then_1
            (goto _label Reset)))))))

(fn ConstructionScript)